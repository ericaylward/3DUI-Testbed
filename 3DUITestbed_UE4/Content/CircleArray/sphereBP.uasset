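; Target sphere actor for a circle array that is selected by a trigger click through raycast or controller overlap.
; The level script activates it, and its material shows target, hover, selected or externally flagged misclick states.
; Hover comes from raycast events or overlap with components tagged "overlapper".
; A click on the active sphere reports itself and the hit position relative to its center back to the level script.
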(event `self.ReceiveBeginPlay`
  ;[1 1 1] Refs
  (bind _outactors (`GameplayStatics.GetAllActorsOfClass` "/Script/Engine.LevelScriptActor"))
  (set `self.levelRef` (`KismetArrayLibrary.Array_Get` _outactors)))

(event `/Game/CircleArray/levelComms.misclickedMatChange`
  (if (`self.isMisclicked`)
    (`PrimitiveComponent.SetMaterial` (`self.sphereMesh`) 0 "/Game/CircleArray/sphereMisclicked.sphereMisclicked")))

(event `/Game/CircleArray/characterComms.triggerClickedOnActor`
  (params (worldPosition_hit :type "Vector Structure"))
  ;[1 1 1] Trigger clicked on sphere (raycast or overlap)
  (`self.Calculate Hit Location` worldPosition_hit)
  (if (`self.isActive`)
    (message `/Game/CircleArray/levelComms.sphereToLevel` (`self.levelRef`) self (`self.relativePos`))
    (`PrimitiveComponent.SetMaterial` (`self.sphereMesh`) 0 "/Game/CircleArray/sphereSelected.sphereSelected")))

(event `/Game/CircleArray/characterComms.raycastBeginOverlap`
  ;[1 1 1] Material changes if touched by raycast
  (if (`self.isActive`)
    (set `self.isOverlapped_ray` true)
    (`PrimitiveComponent.SetMaterial` (`self.sphereMesh`) 0 "/Game/CircleArray/sphereOverlapped.sphereOverlapped")))

(event `/Game/CircleArray/characterComms.raycastEndOverlap`
  ;[1 1 1] Material changes if touched by raycast
  (if (`self.isActive`)
    (set `self.isOverlapped_ray` false)
    (`PrimitiveComponent.SetMaterial` (`self.sphereMesh`) 0 "/Game/CircleArray/sphereTarget.sphereTarget")))

(event `/Game/CircleArray/levelComms.levelToSphere_makeActive`
  ;[1 1 1] Change material if sphere is active sphere
  (set `self.isActive` true)
  (`PrimitiveComponent.SetMaterial` (`self.sphereMesh`) 0 "/Game/CircleArray/sphereTarget.sphereTarget"))

(event `Calculate Hit Location`
  (params (`World Position Hit` :type "Vector Structure"))
  ;[1 1 1] Finds relative position of hit location on sphere
  (bind _output_get (set `self.sphereWorldPos` (`SceneComponent.K2_GetComponentLocation` (`self.sphereMesh`))))
  (bind _output_get_2 (set `self.hitWorldPos` `World Position Hit`))
  (set `self.relativePos` (- _output_get_2 _output_get)))

(event `self.sphereMesh.OnComponentBeginOverlap`
  (params (OverlappedComponent :type "PrimitiveComponent Object Reference") (OtherActor :type "Actor Object Reference") (OtherComp :type "PrimitiveComponent Object Reference") (OtherBodyIndex :type Integer) (bFromSweep :type Boolean) (SweepResult :type "HitResult Structure (by ref)"))
  ;[1 1 1] Material changes if overlapped by controller
  (if (`ActorComponent.ComponentHasTag` OtherComp "overlapper")
    (if (`self.isActive`)
      (`PrimitiveComponent.SetMaterial` (`self.sphereMesh`) 0 "/Game/CircleArray/sphereOverlapped.sphereOverlapped"))))

(event `self.sphereMesh.OnComponentEndOverlap`
  (params (OverlappedComponent :type "PrimitiveComponent Object Reference") (OtherActor :type "Actor Object Reference") (OtherComp :type "PrimitiveComponent Object Reference") (OtherBodyIndex :type Integer))
  ;[1 1 1] Material changes if overlapped by controller
  (if (`ActorComponent.ComponentHasTag` OtherComp "overlapper")
    (if (`self.isActive`)
      (`PrimitiveComponent.SetMaterial` (`self.sphereMesh`) 0 "/Game/CircleArray/sphereTarget.sphereTarget"))))

(fn `UserConstructionScript`)