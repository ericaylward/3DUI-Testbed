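; Spawner for a VR interaction test that builds rings of spheres, with optional cylinders and an enclosing box.
; SessionNumber picks one of ten presets for size, radius and depth; NextPermutation clears spheres and cylinders, then respawns.
; A rotated SpawnSphere component places each actor by local offset, then depth is staggered cumulatively or on alternate items.
; It sends interaction mode to the VR pawn, and spheres, session variables and test start to the level script.
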(event `begin play`
  (bind _spherediameter_incm (`self.SphereDiameter_inCM`))
  (bind _diameter_array (`self.diameter_array`))
  (bind _depth_array (`self.depth_array`))
  (bind _cylinderheight_array (`self.cylinderHeight_array`))
  (bind _centerdistance_array (`self.centerDistance_array`))
  (bind _depthtype (`self.depthType`))
  (bind _item (`KismetArrayLibrary.Array_Get` _centerdistance_array 2))
  (bind _item_2 (`KismetArrayLibrary.Array_Get` _diameter_array))
  (bind _item_3 (`KismetArrayLibrary.Array_Get` _depth_array))
  (bind _item_4 (`KismetArrayLibrary.Array_Get` _cylinderheight_array))
  (bind _item_5 (`KismetArrayLibrary.Array_Get` _centerdistance_array))
  (bind _item_6 (`KismetArrayLibrary.Array_Get` _depthtype))
  (bind _item_7 (`KismetArrayLibrary.Array_Get` _cylinderheight_array 1))
  (bind _item_8 (`KismetArrayLibrary.Array_Get` _centerdistance_array 1))
  (bind _item_9 (`KismetArrayLibrary.Array_Get` _diameter_array 1))
  (bind _item_10 (`KismetArrayLibrary.Array_Get` _depth_array 1))
  (bind _item_11 (`KismetArrayLibrary.Array_Get` _depthtype 2))
  (set `self.sessionNumber` 0)
  (`self.Reset All` :!label _label)
  (`KismetSystemLibrary.Delay` 0.6)
  (switch `int` (stale `/Game/CircleArray/levelComms.nextPermutation` _output_get)
    (:`0`
      (set `self.SphereDiameter_inCM` _item_2)
      (set `self.SphereDepth_inCM` _item_3)
      (set `self.CylinderHeight_inCM` _item_4)
      (set `self.SphereDistFromCenter_inCM` _item_5)
      (set `self.depth_offset_type` _item_11))
    (:`1`
      (set `self.SphereDiameter_inCM` _item_9)
      (set `self.SphereDepth_inCM` _item_3)
      (set `self.CylinderHeight_inCM` _item_7)
      (set `self.SphereDistFromCenter_inCM` _item_5)
      (set `self.depth_offset_type` _item_11))
    (:`2`
      (set `self.SphereDiameter_inCM` _item_2)
      (set `self.SphereDepth_inCM` _item_3)
      (set `self.CylinderHeight_inCM` _item_7)
      (set `self.SphereDistFromCenter_inCM` _item_5)
      (set `self.depth_offset_type` _item_11))
    (:`3`
      (set `self.SphereDiameter_inCM` _item_2)
      (set `self.SphereDepth_inCM` _item_10)
      (set `self.CylinderHeight_inCM` _item_7)
      (set `self.SphereDistFromCenter_inCM` _item_8)
      (set `self.depth_offset_type` _item_11))
    (:`4`
      (set `self.SphereDiameter_inCM` _item_9)
      (set `self.SphereDepth_inCM` _item_10)
      (set `self.CylinderHeight_inCM` _item_4)
      (set `self.SphereDistFromCenter_inCM` _item_8)
      (set `self.depth_offset_type` _item_6))
    (:`5`
      (set `self.SphereDiameter_inCM` _item_9)
      (set `self.SphereDepth_inCM` _item_10)
      (set `self.CylinderHeight_inCM` _item_4)
      (set `self.SphereDistFromCenter_inCM` _item)
      (set `self.depth_offset_type` _item_6))
    (:`6`
      (set `self.SphereDiameter_inCM` _item_9)
      (set `self.SphereDepth_inCM` _item_10)
      (set `self.CylinderHeight_inCM` _item_7)
      (set `self.SphereDistFromCenter_inCM` _item)
      (set `self.depth_offset_type` _item_11))
    (:`7`
      (set `self.SphereDiameter_inCM` _item_9)
      (set `self.SphereDepth_inCM` _item_3)
      (set `self.CylinderHeight_inCM` _item_7)
      (set `self.SphereDistFromCenter_inCM` _item_5)
      (set `self.depth_offset_type` _item_11))
    (:`8`
      (set `self.SphereDiameter_inCM` _item_9)
      (set `self.SphereDepth_inCM` _item_3)
      (set `self.CylinderHeight_inCM` _item_4)
      (set `self.SphereDistFromCenter_inCM` _item_8)
      (set `self.depth_offset_type` _item_11))
    (:`9`
      (set `self.SphereDiameter_inCM` _item_9)
      (set `self.SphereDepth_inCM` _item_3)
      (set `self.CylinderHeight_inCM` _item_4)
      (set `self.SphereDistFromCenter_inCM` _item)
      (set `self.depth_offset_type` _item_6)))
  (set `self.ScaleSphere` (`KismetMathLibrary.MakeVector` _spherediameter_incm _spherediameter_incm _spherediameter_incm))
  (set `self.SphereDistVector` (`KismetMathLibrary.MakeVector` 0.0 0.0 (`self.SphereDistFromCenter_inCM`)))
  (`self.Begin Spawn`))

(event `/Game/CircleArray/levelComms.nextPermutation`
  (params (sessionNum :type Integer))
  (bind _output_get (set `self.sessionNumber` sessionNum))
  (goto _label))

(event `Reset All`
  (message `/Game/CircleArray/characterComms.interactionDelay` (`self.playerRef`))
  (`KismetSystemLibrary.Delay` 0.25)
  (bind _outactors (`GameplayStatics.GetAllActorsOfClass` "/Game/CircleArray/sphereBP.sphereBP_C"))
  (bind _outactors_2 (`GameplayStatics.GetAllActorsOfClass` "/Game/CircleArray/cylinderBP.cylinderBP_C"))
  (`self.K2_DestroyActor` _outactors)
  (`self.K2_DestroyActor` _outactors_2)
  (set `self.SphereDiameter_inCM` 0.0)
  (set `self.SphereDepth_inCM` 0.0)
  (set `self.SphereDistFromCenter_inCM` 0.0)
  (set `self.CylinderHeight_inCM` 0.0)
  (set `self.depth_offset_type` "None"))

(event `self.ReceiveBeginPlay`
  (bind _spherediameter_incm (`self.SphereDiameter_inCM`))
  (bind _spheredistfromcenter_incm (`self.SphereDistFromCenter_inCM`))
  (bind _returnvalue (+ _spheredistfromcenter_incm 10.0))
  ;[1 1 1] Initialization
  (bind _outactors (`GameplayStatics.GetAllActorsOfClass` "/Game/Player/VR_Pawn.VR_Pawn_C"))
  (bind _output_get (set `self.playerRef` (`KismetArrayLibrary.Array_Get` _outactors)))
  (message `/Game/CircleArray/levelComms.spawnerToPlayer` _output_get (`self.raycast_or_overlap`))
  (bind _outactors_2 (`GameplayStatics.GetAllActorsOfClass` "/Script/Engine.LevelScriptActor"))
  (set `self.levelRef` (`KismetArrayLibrary.Array_Get` _outactors_2))
  (`self.ToggleShadow`)
  (set `self.RotatorIncrease` (/ (`self.360`) (`KismetMathLibrary.Conv_IntToDouble` (`self.CirclesToSpawn`))))
  (set `self.ScaleSphere` (`KismetMathLibrary.MakeVector` _spherediameter_incm _spherediameter_incm _spherediameter_incm))
  (set `self.SphereDistVector` (`KismetMathLibrary.MakeVector` 0.0 0.0 _spheredistfromcenter_incm))
  (set `self.BoxScale` (`KismetMathLibrary.MakeVector` _returnvalue _returnvalue _returnvalue))
  (`ActorComponent.K2_DestroyComponent` (`self.PaperSprite`))
  (`self.begin play`))

(event `Begin Spawn`
  ;[1 1 1] Spawn setup
  (for _index (range (`self.CirclesToSpawn`))
    (bind _output_get (set `self.Rotator` (`KismetMathLibrary.MakeRotator` (* _index (* (`self.RotatorIncrease`) -1.0)))))
    (`SceneComponent.K2_SetWorldRotation` (`self.spawnSphere`) _output_get false false)
    (`|ExecutionSequence`
      (:`then_0`
        (`self.Spawn Sphere`))
      (:`then_1`
        (`self.Spawn Cylinder`))))
  (bind _outactors (`GameplayStatics.GetAllActorsOfClass` "/Game/CircleArray/sphereBP.sphereBP_C"))
  (set `self.sphereBP_Array` _outactors)
  (bind _outactors_2 (`GameplayStatics.GetAllActorsOfClass` "/Game/CircleArray/cylinderBP.cylinderBP_C"))
  (set `self.cylinderBP_Array` _outactors_2)
  (`self.sessionVariables` (`self.CirclesToSpawn`) (`self.SphereDiameter_inCM`) (`self.SphereDepth_inCM`) (`self.SphereDistFromCenter_inCM`) (`self.CylinderHeight_inCM`) (`self.raycast_or_overlap`) (`self.depth_offset_type`) (`self.spawnBox?`) (`self.spawnCylinder?`) (`self.shadows?`))
  (`|ExecutionSequence`
    (:`then_0`
      (`self.setDepth`)
      (message `/Game/CircleArray/levelComms.beginTest` (`self.levelRef`))
      (`SceneComponent.ResetRelativeTransform` (`self.spawnSphere`)))
    (:`then_1`
      (`self.Spawn Box`))))

(event `setDepth`
  (bind _spheredepth_incm (`self.SphereDepth_inCM`))
  (bind _spheredepth_init (`self.sphereDepth_init`))
  ;[1 1 1] Sets depth offset
  (switch `name` (`self.depth_offset_type`)
    (:`additive`
      (for (_array_element _array_index) (`self.sphereBP_Array`)
        (`self.K2_AddActorLocalOffset` _array_element (`KismetMathLibrary.MakeVector` _spheredepth_init) false false)
        (`self.K2_AddActorLocalOffset` (`KismetArrayLibrary.Array_Get` (`self.cylinderBP_Array`) _array_index) (`KismetMathLibrary.MakeVector` _spheredepth_init) false false)
        (set `self.sphereDepth_init` (+ (`self.SphereDepth_inCM`) (`self.sphereDepth_init`)))))
    (:`everyother`
      (for (_array_element_2 _array_index_2) (`self.sphereBP_Array`)
        (if (== (mod _array_index_2 2) 0)
          (`self.K2_AddActorLocalOffset` _array_element_2 (`KismetMathLibrary.MakeVector` _spheredepth_incm) false false)
          (`self.K2_AddActorLocalOffset` (`KismetArrayLibrary.Array_Get` (`self.cylinderBP_Array`) _array_index_2) (`KismetMathLibrary.MakeVector` _spheredepth_incm) false false))))))

(event `Spawn Sphere`
  ;[1 1 1] Spawns Spheres
  (bind _returnvalue (`|SpawnActorFromClass` "/Game/CircleArray/sphereBP.sphereBP_C" (`SceneComponent.K2_GetComponentToWorld` (`self.spawnSphere`)) "AlwaysSpawn" "OverrideRootScale"))
  (`self.K2_AddActorLocalOffset` _returnvalue (`self.SphereDistVector`) false false)
  (`SceneComponent.SetWorldScale3D` (`/Game/CircleArray/sphereBP.sphereMesh` _returnvalue) (`self.ScaleSphere`))
  (message `/Game/CircleArray/levelComms.spawnerToLevel` (`self.levelRef`) _returnvalue (`self.sphereToStart`)))

(event `Spawn Cylinder`
  (bind (_scalesphere_x _scalesphere_y _scalesphere_z) (`KismetMathLibrary.BreakVector` (`self.ScaleSphere`)))
  ;[1 1 1] Spawns Cylinders
  (if (`self.spawnCylinder?`)
    (bind _returnvalue (`|SpawnActorFromClass` "/Game/CircleArray/cylinderBP.cylinderBP_C" (`SceneComponent.K2_GetComponentToWorld` (`self.spawnSphere`)) "AlwaysSpawn" "OverrideRootScale"))
    (`self.K2_AddActorLocalOffset` _returnvalue (`self.SphereDistVector`) false false)
    (`SceneComponent.SetWorldScale3D` (`/Game/CircleArray/cylinderBP.cylinderMesh` _returnvalue) (`KismetMathLibrary.MakeVector` (+ (`self.CylinderHeight_inCM`) _scalesphere_x) _scalesphere_y _scalesphere_z))))

(event `ToggleShadow`
  ;[1 1 1] Sets "cast shadow" on/off for directional light
  (message `/Game/CircleArray/levelComms.shadowToggle` (`self.levelRef`) (`self.shadows?`)))

(event `Session Variables - Send to Level`
  (params (circlesToSpawn :type Integer) (sphereDiameter :type "Float (double-precision)") (sphereDepth :type "Float (double-precision)") (sphereDistFromCenter :type "Float (double-precision)") (CylinderHeight :type "Float (double-precision)") (interactionType :type Name) (depthOffsetType :type Name) (`spawnBox?` :type Boolean) (`spawnCylinder?` :type Boolean) (`shadows?` :type Boolean))
  ;[1 1 1] Send level session's variables
  (message `/Game/CircleArray/levelComms.sessionVariables` (`self.levelRef`) circlesToSpawn sphereDiameter sphereDepth sphereDistFromCenter CylinderHeight interactionType depthOffsetType `spawnBox?` `spawnCylinder?` `shadows?`))

(event `Spawn Box`
  (bind (_returnvalue_location _returnvalue_rotation _returnvalue_scale) (`KismetMathLibrary.BreakTransform` (`SceneComponent.K2_GetComponentToWorld` (`self.spawnSphere`))))
  ;[1 1 1] Spawns Box
  (if (`self.spawnBox?`)
    (bind _returnvalue (`|SpawnActorFromClass` "/Game/CircleArray/boxBP.boxBP_C" (`KismetMathLibrary.MakeTransform` _returnvalue_location (struct) _returnvalue_scale) "AlwaysSpawn" "OverrideRootScale"))
    (`SceneComponent.SetWorldScale3D` (`/Game/CircleArray/boxBP.boxMesh` _returnvalue) (`self.BoxScale`))))

(fn `UserConstructionScript`)